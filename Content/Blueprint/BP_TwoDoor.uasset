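; BP_TwoDoor is a double door that swings both leaves open in opposite directions when its OpenDoor event fires.
; A Sequence starts one timeline per door component, restarting the right one but only playing the left one forward.
; Each update lerps that leaf's relative yaw from its current value toward OpenAngle, negated for the left, so easing compounds rather than following the curve directly.
; The graph has no closing logic.
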(event EventBeginPlay)

(event Collision|EventActorBeginOverlap
  (params (OtherActor :type Actor%20Object%20Reference)))

(event EventTick
  (params (DeltaSeconds :type Float%20%28single-precision%29)))

(event EventOpenDoor
  (Utilities|FlowControl|Sequence
    (:then_0
      (bind _openstate (Timeline|TL_OpenDoor PlayFromStart)
        (:Update
          (Transformation|SetRelativeRotation (Variables|Default|GetDoorRightComponent) (Math|Rotator|MakeRotator 0.0 0.0 (Math|Float|Lerp (.Yaw (Math|Rotator|BreakRotator (Variables|/Script/Engine.SceneComponent|GetRelativeRotation (Variables|Default|GetDoorRightComponent)))) (Variables|Default|GetOpenAngle) _openstate)) false false))))
    (:then_1
      (bind _openstate_2 (Timeline|Timeline_0 Play)
        (:Update
          (Transformation|SetRelativeRotation (Variables|Default|GetDoorLeftComponent) (Math|Rotator|MakeRotator 0.0 0.0 (Math|Float|Lerp (.Yaw (Math|Rotator|BreakRotator (Variables|/Script/Engine.SceneComponent|GetRelativeRotation (Variables|Default|GetDoorLeftComponent)))) (* (Variables|Default|GetOpenAngle) -1.0) _openstate_2)) false false))))))

(fn ConstructionScript)